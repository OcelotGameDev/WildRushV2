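; Player 1 pawn for a two-player 2D game of carrying items to delivery points for score, with dashing and attacks that make Player 2 drop items.
; Capsule overlaps handle pickup and delivery, while actor overlap during an attack triggers Player 2's fall.
; Movement updates directional flipbooks by lifting, attacking, falling or walking state, using color-selected arrays.
; It also relays shared-keyboard Player 2 input to BP_PlayerPawn2.
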(event `self.ReceiveBeginPlay`
  (`self.P1SetColor` "NewEnumerator0"))

(event `InputAxis|Moving Up`
  (params (AxisValue :type "Float (single-precision)"))
  ;[0.5219 0.4948 1] Movement
  (bind _output_get (set `self.MoveDirection` (0.0 0.0 1.0)))
  (`self.AddMovementInput` (* (`KismetMathLibrary.Normal` _output_get) (`self.NegateMovementOnAtack`)) AxisValue)
  (`self.PlayFlipbook` :!label _label))

(event `InputAxis|MovingSides`
  (params (AxisValue :type "Float (single-precision)"))
  ;[0.5219 0.4948 1] Movement
  (bind _output_get (set `self.MoveDirection` (1.0 0.0 0.0)))
  (`self.AddMovementInput` (* (`KismetMathLibrary.Normal` _output_get) (`self.NegateMovementOnAtack`)) AxisValue)
  (goto _label))

(event `self.Capsule.OnComponentBeginOverlap`
  (params (OverlappedComponent :type "PrimitiveComponent Object Reference") (OtherActor :type "Actor Object Reference") (OtherComp :type "PrimitiveComponent Object Reference") (OtherBodyIndex :type Integer) (bFromSweep :type Boolean) (SweepResult :type "HitResult Structure (by ref)"))
  (bind _returnvalue (`self.K2_GetActorLocation`))
  (bind _holdingitem (`self.HoldingItem`))
  ;[0.5219 0.4948 1] Comment
  (`|ExecutionSequence`
    (:`then_0`
      (bind _asitem_base (cast `/Game/Blueprints/Item_Base` OtherActor))
      (`|ExecutionSequence`
        (:`then_0`
          (if (not _holdingitem)
            (`PaperSpriteComponent.SetSprite` (`self.ItemSprite`) (`PaperSpriteComponent.GetSprite` (`/Game/Blueprints/Item_Base.Sprite Item` _asitem_base)))
            (set `self.ItemValue` (+ (`/Game/Blueprints/Item_Base.Value` _asitem_base) (`self.ItemValue`)))
            (set `self.isLifting` true)
            (set `self.HoldingItem` true)
            (`GameplayStatics.PlaySoundAtLocation` "/Game/Audio/Samples/Sons_In-Game/Item_Pickup.Item_Pickup" _returnvalue (struct) 1.0 1.0 0.0 null null null)
            (`self.K2_DestroyActor` _asitem_base)))
        (:`then_1`
          (if _holdingitem
            (set `self.currentItem` (`/Game/Blueprints/Item_Base.IndexForSwitch` _asitem_base))))))
    (:`then_1`
      (cast `/Game/Blueprints/DeliverPoint` OtherActor)
      (set `self.PlayerSum` (+ (`self.ItemValue`) (`self.PlayerSum`)))
      (`PaperSpriteComponent.SetSprite` (`self.ItemSprite`) null)
      (set `self.ItemValue` 0)
      (set `self.isLifting` false)
      (`GameplayStatics.PlaySoundAtLocation` "/Game/Audio/Samples/Sons_In-Game/Item_Pickup.Item_Pickup" _returnvalue (struct) 1.0 1.0 0.0 null null null))))

(event `DropP1`
  ;[0.5219 0.4948 1] Comment
  (if (`self.falling`)
    (bind _returnvalue (`|SpawnActorFromClass` "/Game/Blueprints/Item_Base.Item_Base_C" (`KismetMathLibrary.MakeTransform` (`self.K2_GetActorLocation`)) "Undefined" "OverrideRootScale" null null))
    (set `/Game/Blueprints/Item_Base.IndexForSwitch` (`self.currentItem`) _returnvalue)
    (set `self.ItemValue` 0)))

(event `self.ReceiveActorBeginOverlap`
  (params (OtherActor :type "Actor Object Reference"))
  ;[0.4332 0.401 1] Collision To Attack Target
  (bind _asbp_player_pawn_2 (cast `/Game/Blueprints/BP_PlayerPawn2` OtherActor))
  (if (`self.Attacking`)
    (set `/Game/Blueprints/BP_PlayerPawn2.isFalling` true _asbp_player_pawn_2)
    (`/Game/Blueprints/BP_PlayerPawn2.Drop` _asbp_player_pawn_2)))

(event `InputAxis|ArrowUp`
  (params (AxisValue :type "Float (single-precision)"))
  ;[1 0.4271 0.4271] Comment
  (if (`self.unPaused?`)
    (bind _outactors (`GameplayStatics.GetAllActorsOfClass` "/Game/Blueprints/BP_PlayerPawn2.BP_PlayerPawn2_C"))
    (`/Game/Blueprints/InputToP2.CallInputToP2UP` _outactors AxisValue)
    (`/Game/Blueprints/InputToP2.PlaySoundSteps` _outactors (`self.GetInputAxisValue`) (`self.GetInputAxisValue`))))

(event `InputAxis|ArrowRight`
  (params (AxisValue :type "Float (single-precision)"))
  ;[1 0.4271 0.4271] Comment
  (if (`self.unPaused?`)
    (bind _outactors (`GameplayStatics.GetAllActorsOfClass` "/Game/Blueprints/BP_PlayerPawn2.BP_PlayerPawn2_C"))
    (`/Game/Blueprints/BP_PlayerPawn2.CallInputToP2Sides` _outactors AxisValue)
    (`/Game/Blueprints/InputToP2.PlaySoundSteps` _outactors (`self.GetInputAxisValue`) (`self.GetInputAxisValue`))))

(event `Key|RightShift`
  (params (Key :type "Key Structure"))
  ;[1 0.4271 0.4271] Comment
  (:`Pressed`
    (set `self.DashP2` 0.0)
    (bind _returnvalue (`GameplayStatics.GetActorOfClass` "/Game/Blueprints/BP_PlayerPawn2.BP_PlayerPawn2_C"))
    (`/Game/Blueprints/InputToP2.CallDashToP2` _returnvalue (`self.DashP2`)))
  (:`Released`
    (set `self.DashP2` 0.0)))

(event `Key|LeftShift`
  (params (Key :type "Key Structure"))
  ;[0.5219 0.4948 1] Dash
  (:`Pressed`
    (`self.DashCount`))
  (:`Released`
    (set `FloatingPawnMovement.MaxSpeed` 100.0 (`self.FloatingPawnMovement`))))

(event `PlayerAudio`
  (bind _audio (`self.Audio`))
  (if (or (!= (`self.GetInputAxisValue`) 0.0) (!= (`self.GetInputAxisValue`) 0.0))
    (`AudioComponent.Play` _audio 0.0)
    (else
      (`AudioComponent.Stop` _audio))))

(event `Key|RightControl`
  (params (Key :type "Key Structure"))
  ;[1 0.4271 0.4271] Comment
  (:`Pressed`
    (set `self.AttackINGp2` true)
    (bind _returnvalue (`GameplayStatics.GetActorOfClass` "/Game/Blueprints/BP_PlayerPawn2.BP_PlayerPawn2_C"))
    (`/Game/Blueprints/InputToP2.CallAttackToP2` _returnvalue (`self.AttackINGp2`) :!label _label_2))
  (:`Released`
    (set `self.AttackINGp2` false)
    (goto _label_2)))

(event `DashCount`
  (bind _dashcounter (`self.dashCounter`))
  ;[0.5219 0.4948 1] Dash
  (if (> _dashcounter 0)
    (bind _result (`/Engine/EditorBlueprintResources/StandardMacros.DecrementInt` _dashcounter)
      (:`  `
        (set `self.dashCounter` _result)
        (set `FloatingPawnMovement.MaxSpeed` 150.0 (`self.FloatingPawnMovement`))))))

(event `Key|E`
  (params (Key :type "Key Structure"))
  ;[0.4332 0.401 1] Comment
  (:`Pressed`
    (`self.AtkCount`))
  (:`Released`
    (set `self.Attacking` false)))

(event `Key|W`
  (params (Key :type "Key Structure"))
  ;[0.5219 0.4948 1] Comment
  (:`Pressed`
    (`self.PlayerAudio` :!label _label_3))
  (:`Released`
    (goto _label_3)))

(event `Key|D`
  (params (Key :type "Key Structure"))
  ;[0.5219 0.4948 1] Comment
  (:`Pressed`
    (`self.PlayerAudio` :!label _label_4))
  (:`Released`
    (goto _label_4)))

(event `AtkCount`
  (bind _bumpcounter (`self.bumpCounter`))
  ;[0.4332 0.401 1] Comment
  (set `self.Attacking` true)
  (if (> _bumpcounter 0)
    (bind _result (`/Engine/EditorBlueprintResources/StandardMacros.DecrementInt` _bumpcounter)
      (:`  `
        (set `self.bumpCounter` _result)))
    (else
      (set `self.bumpCounter` 0))))

(event `Key|S`
  (params (Key :type "Key Structure"))
  ;[0.5219 0.4948 1] Comment
  (:`Pressed`
    (`self.PlayerAudio` :!label _label_5))
  (:`Released`
    (goto _label_5)))

(event `Key|A`
  (params (Key :type "Key Structure"))
  ;[0.5219 0.4948 1] Comment
  (:`Pressed`
    (`self.PlayerAudio` :!label _label_6))
  (:`Released`
    (goto _label_6)))

(fn `AttackP2`
  (bind _result (`/Engine/EditorBlueprintResources/StandardMacros.IncrementInt` (`self.bumpCounter`))
    (:`  `
      (set `self.bumpCounter` _result))))

(fn `Drop P2`
  (bind _asbp_player_pawn_2 (cast `/Game/Blueprints/BP_PlayerPawn2` (`GameplayStatics.GetPlayerPawn` 1)))
  (`|SpawnActorFromClass` "/Game/Blueprints/Item_Base.Item_Base_C" (`KismetMathLibrary.MakeTransform` (`SceneComponent.K2_GetComponentLocation` (`/Game/Blueprints/BP_PlayerPawn2.Capsule` _asbp_player_pawn_2))) "Undefined" "OverrideRootScale" null null))

(fn `P1Attack`
  (bind _returnvalue (`self.GetInputAxisValue`))
  (bind _flipbook_array (`self.Flipbook Array`))
  (bind _directionenum (`self.DirectionEnum`))
  (if (or (!= (`self.GetInputAxisValue`) 0.0) (!= (`self.GetInputAxisValue`) 0.0))
    (set `self.DirectionEnum` (select `bool` (> _returnvalue 0.0) :`false` (select `bool` (< _returnvalue 0.0) :`false` (select `bool` (> (`self.GetInputAxisValue`) 0.0) :`false` "NewEnumerator3" :`true` "NewEnumerator2" :!type "/Game/Blueprints/Enum_Direction Enum") :`true` "NewEnumerator1") :`true` "NewEnumerator0")))
  (`PaperFlipbookComponent.SetFlipbook` (`self.PaperFlipbook`) (select `bool` (`self.Attacking`) :`false` (select `/Game/Blueprints/Enum_Direction` _directionenum :`NewEnumerator0` (`|GetArrayItem` _flipbook_array) :`NewEnumerator1` (`|GetArrayItem` _flipbook_array 1) :`NewEnumerator2` (`|GetArrayItem` _flipbook_array 2) :`NewEnumerator3` (`|GetArrayItem` _flipbook_array 3)) :`true` (select `/Game/Blueprints/Enum_Direction` _directionenum :`NewEnumerator0` (`|GetArrayItem` _flipbook_array 16) :`NewEnumerator1` (`|GetArrayItem` _flipbook_array 17) :`NewEnumerator2` (`|GetArrayItem` _flipbook_array 18) :`NewEnumerator3` (`|GetArrayItem` _flipbook_array 19)))))

(fn `P1Falling`
  (bind _returnvalue (`self.GetInputAxisValue`))
  (bind _flipbook_array (`self.Flipbook Array`))
  (bind _directionenum (`self.DirectionEnum`))
  (if (or (!= (`self.GetInputAxisValue`) 0.0) (!= (`self.GetInputAxisValue`) 0.0))
    (set `self.DirectionEnum` (select `bool` (> _returnvalue 0.0) :`false` (select `bool` (< _returnvalue 0.0) :`false` (select `bool` (> (`self.GetInputAxisValue`) 0.0) :`false` "NewEnumerator3" :`true` "NewEnumerator2" :!type "/Game/Blueprints/Enum_Direction Enum") :`true` "NewEnumerator1") :`true` "NewEnumerator0")))
  (`PaperFlipbookComponent.SetFlipbook` (`self.PaperFlipbook`) (select `bool` (`self.falling`) :`false` (select `/Game/Blueprints/Enum_Direction` _directionenum :`NewEnumerator0` (`|GetArrayItem` _flipbook_array) :`NewEnumerator1` (`|GetArrayItem` _flipbook_array 1) :`NewEnumerator2` (`|GetArrayItem` _flipbook_array 2) :`NewEnumerator3` (`|GetArrayItem` _flipbook_array 3)) :`true` (select `/Game/Blueprints/Enum_Direction` _directionenum :`NewEnumerator0` (`|GetArrayItem` _flipbook_array 20) :`NewEnumerator1` (`|GetArrayItem` _flipbook_array 21) :`NewEnumerator2` (`|GetArrayItem` _flipbook_array 22) :`NewEnumerator3` (`|GetArrayItem` _flipbook_array 23)))))

(fn `P1Lifting`
  (bind _returnvalue (`self.GetInputAxisValue`))
  (bind _flipbook_array (`self.Flipbook Array`))
  (bind _directionenum (`self.DirectionEnum`))
  (if (or (!= (`self.GetInputAxisValue`) 0.0) (!= (`self.GetInputAxisValue`) 0.0))
    (set `self.DirectionEnum` (select `bool` (> _returnvalue 0.0) :`false` (select `bool` (< _returnvalue 0.0) :`false` (select `bool` (> (`self.GetInputAxisValue`) 0.0) :`false` "NewEnumerator3" :`true` "NewEnumerator2" :!type "/Game/Blueprints/Enum_Direction Enum") :`true` "NewEnumerator1") :`true` "NewEnumerator0")))
  (`PaperFlipbookComponent.SetFlipbook` (`self.PaperFlipbook`) (select `bool` (> (`KismetMathLibrary.VSize` (`SceneComponent.GetComponentVelocity` (`self.Capsule`))) 0.2) :`false` (select `/Game/Blueprints/Enum_Direction` _directionenum :`NewEnumerator0` (`|GetArrayItem` _flipbook_array 8) :`NewEnumerator1` (`|GetArrayItem` _flipbook_array 9) :`NewEnumerator2` (`|GetArrayItem` _flipbook_array 10) :`NewEnumerator3` (`|GetArrayItem` _flipbook_array 11)) :`true` (select `/Game/Blueprints/Enum_Direction` _directionenum :`NewEnumerator0` (`|GetArrayItem` _flipbook_array 12) :`NewEnumerator1` (`|GetArrayItem` _flipbook_array 13) :`NewEnumerator2` (`|GetArrayItem` _flipbook_array 14) :`NewEnumerator3` (`|GetArrayItem` _flipbook_array 15)))))

(fn `P1SetColor`
  (params (Selection :type "/Game/Blueprints/Enum_Flipbooks Enum" :default "NewEnumerator0"))
  (switch `/Game/Blueprints/Enum_Flipbooks` Selection
    (:`NewEnumerator0`
      (set `self.Flipbook Array` (`self.Fbks_Red`)))
    (:`NewEnumerator1`
      (set `self.Flipbook Array` (`self.Fbks_Green`)))
    (:`NewEnumerator2`
      (set `self.Flipbook Array` (`self.Fbks_Blue`)))
    (:`NewEnumerator3`
      (set `self.Flipbook Array` (`self.Fbks_Yellow`)))))

(fn `P1Walking`
  (bind _returnvalue (`self.GetInputAxisValue`))
  (bind _flipbook_array (`self.Flipbook Array`))
  (bind _directionenum (`self.DirectionEnum`))
  (if (or (!= (`self.GetInputAxisValue`) 0.0) (!= (`self.GetInputAxisValue`) 0.0))
    (set `self.isWalking` true)
    (set `self.DirectionEnum` (select `bool` (> _returnvalue 0.0) :`false` (select `bool` (< _returnvalue 0.0) :`false` (select `bool` (> (`self.GetInputAxisValue`) 0.0) :`false` "NewEnumerator3" :`true` "NewEnumerator2" :!type "/Game/Blueprints/Enum_Direction Enum") :`true` "NewEnumerator1") :`true` "NewEnumerator0"))
    (else
      (set `self.isWalking` false)))
  (`PaperFlipbookComponent.SetFlipbook` (`self.PaperFlipbook`) (select `bool` (> (`KismetMathLibrary.VSize` (`SceneComponent.GetComponentVelocity` (`self.Capsule`))) 0.0) :`false` (select `/Game/Blueprints/Enum_Direction` _directionenum :`NewEnumerator0` (`|GetArrayItem` _flipbook_array) :`NewEnumerator1` (`|GetArrayItem` _flipbook_array 1) :`NewEnumerator2` (`|GetArrayItem` _flipbook_array 2) :`NewEnumerator3` (`|GetArrayItem` _flipbook_array 3)) :`true` (select `/Game/Blueprints/Enum_Direction` _directionenum :`NewEnumerator0` (`|GetArrayItem` _flipbook_array 4) :`NewEnumerator1` (`|GetArrayItem` _flipbook_array 5) :`NewEnumerator2` (`|GetArrayItem` _flipbook_array 6) :`NewEnumerator3` (`|GetArrayItem` _flipbook_array 7)))))

(fn `PlayFlipbook`
  (if (`self.isLifting`)
    (`self.P1Lifting`)
    (elif (`self.Attacking`)
      (`self.P1Attack`)
      (elif (`self.falling`)
        (`self.P1Falling`)
        (else
          (`self.P1Walking`))))))

(fn `UserConstructionScript`)