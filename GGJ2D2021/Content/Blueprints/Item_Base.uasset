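; Item_Base is an item Blueprint with a sprite, value and weight, covering types such as food, treasure and western-themed objects.
; On BeginPlay, a switch on IndexForSwitch calls a per-type event with array index 0.
; Each event reassigns Value and Weight to themselves and sets SpriteItem from NewSource.
; Beer's event is empty beside an unconnected copy of that logic, and the construction script and ConstantLocation are empty.
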(event `self.ReceiveBeginPlay`
  (switch `int` (`self.IndexForSwitch`)
    (:`0`
      (`self.Meat` 0))
    (:`1`
      (`self.Vial` 0))
    (:`2`
      (`self.Gold` 0))
    (:`3`
      (`self.Chicken` 0))
    (:`4`
      (`self.Beer` 0))
    (:`5`
      (`self.Cards` 0))
    (:`6`
      (`self.Gaita` 0))
    (:`7`
      (`self.MoneyBag` 0))
    (:`8`
      (`self.Diamond` 0))
    (:`9`
      (`self.Gun` 0))
    (:`10`
      (`self.Star` 0))
    (:`11`
      (`self.Hat` 0))
    (:`12`
      (`self.Cartaz` 0))
    (:`13`
      (`self.Bota` 0))
    (:`14`
      (`self.ShoeHorse` 0))))

(event `Meat`
  (params (`arrayIndex 1` :type Integer))
  ;[1 1 1] Comment
  (set `self.Value` (`self.Value`))
  (set `self.Weight` (`self.Weight`))
  (`PaperSpriteComponent.SetSprite` (`self.Sprite Item`) (`|GetArrayItem` (`self.NewSource`) `arrayIndex 1`)))

(event `Cards`
  (params (`arrayIndex 1` :type Integer))
  ;[1 1 1] Comment
  (set `self.Value` (`self.Value`))
  (set `self.Weight` (`self.Weight`))
  (`PaperSpriteComponent.SetSprite` (`self.Sprite Item`) (`|GetArrayItem` (`self.NewSource`) `arrayIndex 1`)))

(event `Star`
  (params (arrayIndex :type Integer))
  ;[1 1 1] Comment
  (set `self.Value` (`self.Value`))
  (set `self.Weight` (`self.Weight`))
  (`PaperSpriteComponent.SetSprite` (`self.Sprite Item`) (`|GetArrayItem` (`self.NewSource`) arrayIndex)))

(event `Vial`
  (params (`arrayIndex 1` :type Integer))
  ;[1 1 1] Comment
  (set `self.Value` (`self.Value`))
  (set `self.Weight` (`self.Weight`))
  (`PaperSpriteComponent.SetSprite` (`self.Sprite Item`) (`|GetArrayItem` (`self.NewSource`) `arrayIndex 1`)))

(event `Gaita`
  (params (`arrayIndex 1` :type Integer))
  ;[1 1 1] Comment
  (set `self.Value` (`self.Value`))
  (set `self.Weight` (`self.Weight`))
  (`PaperSpriteComponent.SetSprite` (`self.Sprite Item`) (`|GetArrayItem` (`self.NewSource`) `arrayIndex 1`)))

(event `Hat`
  (params (arrayIndex :type Integer))
  ;[1 1 1] Comment
  (set `self.Value` (`self.Value`))
  (set `self.Weight` (`self.Weight`))
  (`PaperSpriteComponent.SetSprite` (`self.Sprite Item`) (`|GetArrayItem` (`self.NewSource`) arrayIndex)))

(event `Gold`
  (params (`arrayIndex 1` :type Integer))
  ;[1 1 1] Comment
  (set `self.Value` (`self.Value`))
  (set `self.Weight` (`self.Weight`))
  (`PaperSpriteComponent.SetSprite` (`self.Sprite Item`) (`|GetArrayItem` (`self.NewSource`) `arrayIndex 1`)))

(event `Cartaz`
  (params (arrayIndex :type Integer))
  ;[1 1 1] Comment
  (set `self.Value` (`self.Value`))
  (set `self.Weight` (`self.Weight`))
  (`PaperSpriteComponent.SetSprite` (`self.Sprite Item`) (`|GetArrayItem` (`self.NewSource`) arrayIndex)))

(event `MoneyBag`
  (params (`arrayIndex 1` :type Integer))
  ;[1 1 1] Comment
  (set `self.Value` (`self.Value`))
  (set `self.Weight` (`self.Weight`))
  (`PaperSpriteComponent.SetSprite` (`self.Sprite Item`) (`|GetArrayItem` (`self.NewSource`) `arrayIndex 1`)))

(event `Chicken`
  (params (`arrayIndex 1` :type Integer))
  ;[1 1 1] Comment
  (set `self.Value` (`self.Value`))
  (set `self.Weight` (`self.Weight`))
  (`PaperSpriteComponent.SetSprite` (`self.Sprite Item`) (`|GetArrayItem` (`self.NewSource`) `arrayIndex 1`)))

(event `Bota`
  (params (arrayIndex :type Integer))
  ;[1 1 1] Comment
  (set `self.Value` (`self.Value`))
  (set `self.Weight` (`self.Weight`))
  (`PaperSpriteComponent.SetSprite` (`self.Sprite Item`) (`|GetArrayItem` (`self.NewSource`) arrayIndex)))

(event `Diamond`
  (params (arrayIndex :type Integer))
  ;[1 1 1] Comment
  (set `self.Value` (`self.Value`))
  (set `self.Weight` (`self.Weight`))
  (`PaperSpriteComponent.SetSprite` (`self.Sprite Item`) (`|GetArrayItem` (`self.NewSource`) arrayIndex)))

(event `ShoeHorse`
  (params (arrayIndex :type Integer))
  ;[1 1 1] Comment
  (set `self.Value` (`self.Value`))
  (set `self.Weight` (`self.Weight`))
  (`PaperSpriteComponent.SetSprite` (`self.Sprite Item`) (`|GetArrayItem` (`self.NewSource`) arrayIndex)))

(event `Gun`
  (params (arrayIndex :type Integer))
  ;[1 1 1] Comment
  (set `self.Value` (`self.Value`))
  (set `self.Weight` (`self.Weight`))
  (`PaperSpriteComponent.SetSprite` (`self.Sprite Item`) (`|GetArrayItem` (`self.NewSource`) arrayIndex)))

(event `Beer`
  (params (`arrayIndex 1` :type Integer))
  ;[1 1 1] Comment
)

(fn `Constant Location`)

(fn `UserConstructionScript`)