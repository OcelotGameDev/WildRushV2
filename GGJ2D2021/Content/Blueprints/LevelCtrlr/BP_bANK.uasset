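; Bank building actor that opens up the view of its interior when a pawn passes through its trigger box.
; Each pawn begin-overlap on the Box drives a FlipFlop that alternately hides and shows the FRONT and Roof components.
; The same toggle plays a door opening or closing sound through the Audio component.
; State follows the count of overlaps by any pawn, as there is no end-overlap handling.
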(event `self.ReceiveBeginPlay`)

(event `self.Box.OnComponentBeginOverlap`
  (params (OverlappedComponent :type "PrimitiveComponent Object Reference") (OtherActor :type "Actor Object Reference") (OtherComp :type "PrimitiveComponent Object Reference") (OtherBodyIndex :type Integer) (bFromSweep :type Boolean) (SweepResult :type "HitResult Structure (by ref)"))
  (bind _front (`self.fRONT`))
  (bind _roof (`self.Roof`))
  (bind _audio (`self.Audio`))
  (cast `Pawn` OtherActor)
  (`/Engine/EditorBlueprintResources/StandardMacros.FlipFlop`
    (:`A`
      (`SceneComponent.SetVisibility` _front false false)
      (`SceneComponent.SetVisibility` _roof false false)
      (`AudioComponent.SetSound` _audio "/Game/Audio/Samples/Sons_In-Game/Porta_Abrindo.Porta_Abrindo")
      (`AudioComponent.Play` _audio 0.0))
    (:`B`
      (`SceneComponent.SetVisibility` _front true false)
      (`SceneComponent.SetVisibility` _roof true false)
      (`AudioComponent.SetSound` _audio "/Game/Audio/Samples/Sons_In-Game/Porta_Fechando.Porta_Fechando")
      (`AudioComponent.Play` _audio 0.0))))

(fn `UserConstructionScript`)