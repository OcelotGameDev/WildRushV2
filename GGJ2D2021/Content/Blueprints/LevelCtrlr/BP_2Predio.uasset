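; Building actor that switches between interior and exterior presentation when a pawn triggers its overlap.
; A FlipFlop on begin overlap alternately hides and shows the front and roof meshes, playing door open or close sounds.
; It also swaps the gameplay theme between muffled and normal versions through the LevelCtrl actor found at BeginPlay.
; State follows the overlap count, as no end-overlap check exists.
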(event `self.ReceiveBeginPlay`
  (bind _returnvalue (`GameplayStatics.GetActorOfClass` "/Game/Blueprints/LevelCtrlr/LevelCtrl.LevelCtrl_C"))
  (set `self.referenceLvlCtrl` _returnvalue))

(event `self.ReceiveActorBeginOverlap`
  (params (OtherActor :type "Actor Object Reference"))
  (bind _front (`self.fRONT`))
  (bind _roof (`self.Roof`))
  (bind _audio (`self.Audio`))
  (bind _gameaudio (`/Game/Blueprints/LevelCtrlr/LevelCtrl.GameAudio` (`self.referenceLvlCtrl`)))
  (cast `Pawn` OtherActor)
  (`/Engine/EditorBlueprintResources/StandardMacros.FlipFlop`
    (:`A`
      (`SceneComponent.SetVisibility` _front false false)
      (`SceneComponent.SetVisibility` _roof false false)
      (`AudioComponent.SetSound` _audio "/Game/Audio/Samples/Sons_In-Game/Porta_Abrindo.Porta_Abrindo")
      (`AudioComponent.Play` _audio 0.0)
      (`AudioComponent.SetSound` _gameaudio "/Game/Audio/Musicas__OGG_/Wild_Rush_-_Tema_Gameplay__Abafado_.Wild_Rush_-_Tema_Gameplay__Abafado_"))
    (:`B`
      (`SceneComponent.SetVisibility` _front true false)
      (`SceneComponent.SetVisibility` _roof true false)
      (`AudioComponent.SetSound` _audio "/Game/Audio/Samples/Sons_In-Game/Porta_Fechando.Porta_Fechando")
      (`AudioComponent.Play` _audio 0.0)
      (`AudioComponent.SetSound` _gameaudio "/Game/Audio/Musicas__OGG_/Wild_Rush_-_Tema_Gameplay.Wild_Rush_-_Tema_Gameplay"))))

(fn `UserConstructionScript`)