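; Level controller actor that runs match flow, music and a shared orthographic camera for one or two players.
; It opens on a start menu; unpausing optionally spawns a second pawn, caches player references and takes the view target.
; A self-recalling one-second countdown pauses play and shows the endgame widget at zero.
; A looping timer eases the camera toward the player or pair midpoint, setting zoom from their clamped separation.
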(event `self.ReceiveBeginPlay`
  (bind _gameaudio (`self.GameAudio`))
  (`self.PauseGame`)
  (`AudioComponent.SetSound` _gameaudio "/Game/Audio/Musicas__OGG_/Wild_Rush_-_Tema_Gameplay.Wild_Rush_-_Tema_Gameplay")
  (`AudioComponent.Play` _gameaudio 0.0))

(event `TimerHUD`
  (bind _endgame (`self.endgame`))
  (bind _time (`self.Time`))
  ;[1 1 1] Comment
  (`|ExecutionSequence`
    (:`then_0`
      (if _endgame
        (`self.PauseMidGame`)
        (bind _foundwidgets (`WidgetBlueprintLibrary.GetAllWidgetsOfClass` "/Game/Widgets/Wg_Game.Wg_Game_C" false))
        (`/Game/Widgets/Wg_Game.fVis_Endgame` (`|GetArrayItem` _foundwidgets) _endgame)
        (set `PlayerController.bShowMouseCursor` true (`GameplayStatics.GetPlayerController` 0))
        (`AudioComponent.Stop` (`self.GameAudio`))))
    (:`then_1`
      (if (`self.unpaused?`)
        (if (> _time 0.0)
          (set `self.Time` (- _time 1.0))
          (`GameplayStatics.PlaySound2D` (`self.SoundTick`) 1.0 1.0 0.0 null null)
          (`KismetSystemLibrary.Delay` 1.0)
          (else
            (set `self.endgame` true)))
        (`self.TimerHUD`)))))

(event `UpdateCamera`
  ;[1 1 1] Comment
  (set `CameraComponent.OrthoWidth` (`KismetMathLibrary.FClamp` (`self.GetDistanceTo` (`self.p1Ref`) (`self.p2Ref`)) 512.0 2048.0) (`self.Camera`))
  (`self.UpdateLocation`))

(event `Add Timer`
  ;[1 1 1] Comment
  (bind _returnvalue (`|CreateWidget` "/Game/Widgets/Wg_Game.Wg_Game_C" (`GameplayStatics.GetPlayerController` 0)))
  (`UserWidget.AddToViewport` _returnvalue 0))

(event `NumberOfPlayers`
  ;[1 1 1] Comment
  (bind _outactors (`GameplayStatics.GetAllActorsOfClass` "/Script/Engine.Pawn"))
  (set `self.Players` _outactors))

(event `UpdateLocation`
  ;[1 1 1] Comment
  (if (`self.2pls`)
    (set `self.CameraCurrentPosition` (/ (+ (`self.K2_GetActorLocation` (`self.p1Ref`)) (`self.K2_GetActorLocation` (`self.p2Ref`))) (`KismetArrayLibrary.Array_Length` (`self.Players`))))
    (`self.K2_SetActorLocation` (`KismetMathLibrary.VInterpTo` (`self.PreviousLocation`) (`self.CameraCurrentPosition`) (`GameplayStatics.GetWorldDeltaSeconds`) (`self.LerpSPEED`)))
    (set `self.PreviousLocation` (`self.K2_GetActorLocation` self))
    (else
      (set `self.CameraCurrentPosition` (`self.K2_GetActorLocation` (`self.p1Ref`)))
      (`self.K2_SetActorLocation` (`KismetMathLibrary.VInterpTo` (`self.PreviousLocation`) (`self.CameraCurrentPosition`) (`GameplayStatics.GetWorldDeltaSeconds`) (`self.LerpSPEED`)))
      (set `self.PreviousLocation` (`self.K2_GetActorLocation` self)))))

(fn `GameMode/2Ps`
  (bind _returnvalue (`GameplayStatics.GetActorOfClass` "/Script/Engine.PlayerStart"))
  (`|SpawnActorFromClass` "/Game/Blueprints/BP_PlayerPawn2.BP_PlayerPawn2_C" (`KismetMathLibrary.MakeTransform` (`self.K2_GetActorLocation` _returnvalue)) "Undefined" "OverrideRootScale" null null))

(fn `PauseGame`
  (bind _returnvalue (`GameplayStatics.GetPlayerController` 0))
  (bind _newwgref (`self.NewWGREF`))
  (bind _output_get (set `self.unpaused?` false))
  (if (not _output_get)
    (`/Engine/EditorBlueprintResources/StandardMacros.IsValid` (`self.NewWGREF`)
      (:`Is Valid`
        _)
      (:`Is Not Valid`
        (bind _returnvalue_2 (`|CreateWidget` "/Game/Widgets/Wg_StartPause.Wg_StartPause_C" (`GameplayStatics.GetPlayerController` 0)))
        (set `self.NewWGREF` _returnvalue_2)))
    (`UserWidget.AddToViewport` _newwgref 0)
    (`WidgetBlueprintLibrary.SetInputMode_GameAndUIEx` _returnvalue _newwgref "DoNotLock" false)
    (set `PlayerController.bShowMouseCursor` true _returnvalue)
    (`AudioComponent.SetSound` (`self.GameAudio`) "/Game/Audio/Musicas__OGG_/Wild_Rush_-_Tema_Gameplay.Wild_Rush_-_Tema_Gameplay")))

(fn `PauseMidGame`
  (bind _returnvalue (`GameplayStatics.SetGamePaused` true))
  (if _returnvalue
    (set `self.unpaused?` false)
    (set `PlayerController.bShowMouseCursor` false (`GameplayStatics.GetPlayerController` 0))))

(fn `UnpauseGame`
  (params (Condition :type Boolean))
  (bind _returnvalue (`GameplayStatics.GetPlayerController` 0))
  (bind _gameaudio (`self.GameAudio`))
  (`|ExecutionSequence`
    (:`then_0`
      (set `self.unpaused?` true)
      (`WidgetLayoutLibrary.RemoveAllWidgets`)
      (`WidgetBlueprintLibrary.SetInputMode_GameOnly` _returnvalue)
      (set `PlayerController.bShowMouseCursor` false _returnvalue)
      (if Condition
        (set `self.2pls` true)
        (`self.GameMode/2Ps`)
        (else
          (set `self.2pls` false))))
    (:`then_1`
      (`self.NumberOfPlayers`)
      (`self.TimerHUD`)
      (`AudioComponent.SetSound` _gameaudio "/Game/Audio/Musicas__OGG_/Wild_Rush_-_Tema_Gameplay_2.Wild_Rush_-_Tema_Gameplay_2")
      (`AudioComponent.Play` _gameaudio 0.0)
      (`KismetSystemLibrary.PrintString` "Hello"))
    (:`then_2`
      (bind _returnvalue_2 (`GameplayStatics.GetActorOfClass` "/Script/Engine.PlayerController"))
      (`PlayerController.SetViewTargetWithBlend` _returnvalue_2 self 0.0 "VTBlend_Linear" 0.0 false)
      (for (_array_element _array_index) (`self.Players`)
        (switch `int` _array_index
          (:`0`
            (set `self.p1Ref` _array_element))
          (:`1`
            (set `self.p2Ref` _array_element)))
        (`KismetSystemLibrary.K2_SetTimer` null "UpdateCamera" 0.02 true)))))

(fn `UnpauseMidGame`
  (bind _returnvalue (`GameplayStatics.SetGamePaused` false))
  (if (not _returnvalue)
    (set `self.unpaused?` true)
    (`AudioComponent.SetSound` (`self.GameAudio`) "/Game/Audio/Musicas__OGG_/Wild_Rush_-_Tema_Principal.Wild_Rush_-_Tema_Principal")
    (set `PlayerController.bShowMouseCursor` false (`GameplayStatics.GetPlayerController` 0))))

(fn `UserConstructionScript`)