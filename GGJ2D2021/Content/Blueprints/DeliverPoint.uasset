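; DeliverPoint is a delivery spot that shows a randomly chosen item silhouette from ShadowAway as the current request.
; On BeginPlay it gathers all Item_Base actors, picks a shadow, then polls ItemOnDeliver through a self-calling delay loop.
; When that flag is true, it removes the current entries and picks another shadow, without restarting polling.
; Overlap clears either tagged player's item sprite; the flag is never set here.
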(event `self.ReceiveBeginPlay`
  (bind _outactors (`GameplayStatics.GetAllActorsOfClass` "/Game/Blueprints/Item_Base.Item_Base_C"))
  (set `self.ItensOnSceneRef` _outactors)
  (`self.Spawn Shadow`)
  (`self.Delivering`))

(event `Delivering`
  (bind _current_index (`self.Current Index`))
  ;[1 1 1] Comment
  (if (`self.ItemOnDeliver`)
    (`KismetArrayLibrary.Array_Remove` (`self.Shadow Away`) _current_index)
    (`KismetArrayLibrary.Array_Remove` (`self.ItensOnSceneRef`) _current_index)
    (`KismetSystemLibrary.Delay` 0.02)
    (`self.Spawn Shadow`)
    (else
      (`KismetSystemLibrary.Delay` 0.02)
      (`self.Delivering`))))

(event `Spawn Shadow`
  ;[1 1 1] Comment
  (bind _output_get (set `self.Current Index` (`KismetMathLibrary.RandomIntegerInRange` 0 (- (`KismetArrayLibrary.Array_Length` (`self.ItensOnSceneRef`)) 1))))
  (`PaperSpriteComponent.SetSprite` (`self.Item`) (`|GetArrayItem` (`self.Shadow Away`) _output_get)))

(event `self.DeliCol.OnComponentBeginOverlap`
  (params (OverlappedComponent :type "PrimitiveComponent Object Reference") (OtherActor :type "Actor Object Reference") (OtherComp :type "PrimitiveComponent Object Reference") (OtherBodyIndex :type Integer) (bFromSweep :type Boolean) (SweepResult :type "HitResult Structure (by ref)"))
  (`|ExecutionSequence`
    (:`then_0`
      (if (`self.ActorHasTag` OtherActor "Player1")
        (bind _asbp_player_pawn_1 (cast `/Game/Blueprints/BP_PlayerPawn1` OtherActor))
        (`PaperSpriteComponent.SetSprite` (`/Game/Blueprints/BP_PlayerPawn1.ItemSprite` _asbp_player_pawn_1) null)))
    (:`then_1`
      (if (`self.ActorHasTag` OtherActor "Player2")
        (bind _asbp_player_pawn_2 (cast `/Game/Blueprints/BP_PlayerPawn2` OtherActor))
        (`PaperSpriteComponent.SetSprite` (`/Game/Blueprints/BP_PlayerPawn2.Item Sprite` _asbp_player_pawn_2) null)))))

(fn `UserConstructionScript`)