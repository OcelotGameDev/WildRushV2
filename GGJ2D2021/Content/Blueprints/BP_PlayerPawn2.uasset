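; Player 2's Paper2D pawn in a two-player game of carrying items to delivery points and knocking the rival down.
; Forwarded input events drive X/Z movement, attack, dash and drop, with dropping respawning the carried item.
; Capsule overlaps pick up items and bank their value at DeliverPoints, while attacking sphere overlaps make Player 1 fall and drop.
; PlayFlipbook prioritizes lifting, attack, falling, then walking, picking directional flipbooks from a color-selected array.
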(event `/Game/Blueprints/InputToP2.CallInputToP2UP`
  (params (InputValueZ :type "Float (single-precision)"))
  ;[1 0.4271 0.4271] Comment
  (bind _output_get (set `self.MoveDirection` (0.0 0.0 1.0)))
  (`self.AddMovementInput` (`KismetMathLibrary.Normal` _output_get) InputValueZ)
  (`self.Play Flipbook` InputValueZ (stale `/Game/Blueprints/InputToP2.CallInputToP2Sides` InputValueX) :!label _label))

(event `self.ReceiveBeginPlay`
  ;[1 0.4271 0.4271] Comment
  (`self.SetColor` "NewEnumerator0"))

(event `/Game/Blueprints/InputToP2.CallInputToP2Sides`
  (params (InputValueX :type "Float (single-precision)"))
  ;[1 0.4271 0.4271] Comment
  (bind _output_get (set `self.MoveDirection` (1.0 0.0 0.0)))
  (`self.AddMovementInput` (`KismetMathLibrary.Normal` _output_get) InputValueX)
  (goto _label))

(event `Drop`
  ;[1 0.4271 0.4271] Comment
  (if (`self.isFalling`)
    (bind _returnvalue (`|SpawnActorFromClass` "/Game/Blueprints/Item_Base.Item_Base_C" (`KismetMathLibrary.MakeTransform` (`self.K2_GetActorLocation`)) "Undefined" "OverrideRootScale" null 0 null))
    (set `/Game/Blueprints/Item_Base.IndexForSwitch` (`self.currentItem`) _returnvalue)
    (set `self.HoldingItem` false)))

(event `/Game/Blueprints/InputToP2.CallAttackToP2`
  (params (Attack :type Boolean))
  ;[1 0.4271 0.4271] Comment
  (if Attack
    (`self.AtkCount`)))

(event `/Game/Blueprints/InputToP2.CallDashToP2`
  (params (Dash :type "Float (single-precision)"))
  ;[1 0.4271 0.4271] Comment
  (set `self.DashMx2` Dash))

(event `/Game/Blueprints/InputToP2.PlaySoundSteps`
  (params (Up :type "Float (single-precision)") (Side :type "Float (single-precision)"))
  (bind _audio (`self.Audio`))
  ;[1 0.4271 0.4271] Comment
  (if (or (!= Up 0.0) (!= Side 0.0))
    (`AudioComponent.Play` _audio 0.0)
    (else
      (`AudioComponent.Stop` _audio))))

(event `CallDropToP2_1`
  (params (DropItem :type Boolean))
  ;[1 0.4271 0.4271] Comment
  (set `self.isFalling` DropItem)
  (`self.Drop`))

(event `self.Capsule.OnComponentBeginOverlap`
  (params (OverlappedComponent :type "PrimitiveComponent Object Reference") (OtherActor :type "Actor Object Reference") (OtherComp :type "PrimitiveComponent Object Reference") (OtherBodyIndex :type Integer) (bFromSweep :type Boolean) (SweepResult :type "HitResult Structure (by ref)"))
  (bind _item_sprite (`self.Item Sprite`))
  ;[1 0.4271 0.4271] Comment
  (`|ExecutionSequence`
    (:`then_0`
      (bind _asitem_base (cast `/Game/Blueprints/Item_Base` OtherActor))
      (if (not (`self.HoldingItem`))
        (`PaperSpriteComponent.SetSprite` _item_sprite (`PaperSpriteComponent.GetSprite` (`/Game/Blueprints/Item_Base.Sprite Item` _asitem_base)))
        (set `self.ItemValue` (+ (`/Game/Blueprints/Item_Base.Value` _asitem_base) (`self.ItemValue`)))
        (set `self.isLifting` true)
        (set `self.HoldingItem` true)))
    (:`then_1`
      (set `self.currentItem` (`/Game/Blueprints/Item_Base.IndexForSwitch` _asitem_base)))
    (:`then_2`
      (cast `/Game/Blueprints/DeliverPoint` OtherActor)
      (set `self.PlayerSum` (+ (`self.ItemValue`) (`self.PlayerSum`)))
      (`PaperSpriteComponent.SetSprite` _item_sprite null)
      (`KismetSystemLibrary.Delay` 0.02)
      (set `self.ItemValue` 0)
      (set `self.isLifting` false))))

(event `DashCount`
  (bind _dashcounter (`self.dashCounter`))
  ;[1 0.4271 0.4271] Dash
  (if (> _dashcounter 0)
    (bind _result (`/Engine/EditorBlueprintResources/StandardMacros.DecrementInt` _dashcounter)
      (:`  `
        (set `self.dashCounter` _result)))))

(event `self.Sphere.OnComponentBeginOverlap`
  (params (OverlappedComponent :type "PrimitiveComponent Object Reference") (OtherActor :type "Actor Object Reference") (OtherComp :type "PrimitiveComponent Object Reference") (OtherBodyIndex :type Integer) (bFromSweep :type Boolean) (SweepResult :type "HitResult Structure (by ref)"))
  ;[1 0.4271 0.4271] Collision To Attack Target
  (if (`self.isAttacking`)
    (bind _asbp_player_pawn_1 (cast `/Game/Blueprints/BP_PlayerPawn1` OtherActor))
    (set `/Game/Blueprints/BP_PlayerPawn1.falling` true _asbp_player_pawn_1)
    (`/Game/Blueprints/BP_PlayerPawn1.DropP1` _asbp_player_pawn_1)))

(event `AtkCount`
  (bind _bumpcounter (`self.bumpCounter`))
  ;[1 0.4271 0.4271] Comment
  (set `self.isAttacking` true)
  (if (> _bumpcounter 0)
    (bind _result (`/Engine/EditorBlueprintResources/StandardMacros.DecrementInt` _bumpcounter)
      (:`  `
        (set `self.bumpCounter` _result)))
    (else
      (set `self.bumpCounter` 0))))

(fn `P2Attack`
  (params (ArrowUp :type "Float (double-precision)") (ArrowRight :type "Float (double-precision)"))
  (bind _flipbook_array (`self.Flipbook Array`))
  (bind _directionenum (`self.DirectionEnum`))
  (if (or (!= ArrowUp 0.0) (!= ArrowRight 0.0))
    (set `self.DirectionEnum` (select `bool` (> ArrowUp 0.0) :`false` (select `bool` (< ArrowUp 0.0) :`false` (select `bool` (> ArrowRight 0.0) :`false` "NewEnumerator3" :`true` "NewEnumerator2" :!type "/Game/Blueprints/Enum_Direction Enum") :`true` "NewEnumerator1") :`true` "NewEnumerator0")))
  (`PaperFlipbookComponent.SetFlipbook` (`self.PaperFlipbook`) (select `bool` (`self.isAttacking`) :`false` (select `/Game/Blueprints/Enum_Direction` _directionenum :`NewEnumerator0` (`|GetArrayItem` _flipbook_array) :`NewEnumerator1` (`|GetArrayItem` _flipbook_array 1) :`NewEnumerator2` (`|GetArrayItem` _flipbook_array 2) :`NewEnumerator3` (`|GetArrayItem` _flipbook_array 3)) :`true` (select `/Game/Blueprints/Enum_Direction` _directionenum :`NewEnumerator0` (`|GetArrayItem` _flipbook_array 16) :`NewEnumerator1` (`|GetArrayItem` _flipbook_array 17) :`NewEnumerator2` (`|GetArrayItem` _flipbook_array 18) :`NewEnumerator3` (`|GetArrayItem` _flipbook_array 19)))))

(fn `P2Falling`
  (params (ArrowUp :type "Float (double-precision)") (ArrowRight :type "Float (double-precision)"))
  (bind _flipbook_array (`self.Flipbook Array`))
  (bind _directionenum (`self.DirectionEnum`))
  (if (or (!= ArrowUp 0.0) (!= ArrowRight 0.0))
    (set `self.DirectionEnum` (select `bool` (> ArrowUp 0.0) :`false` (select `bool` (< ArrowUp 0.0) :`false` (select `bool` (> ArrowRight 0.0) :`false` "NewEnumerator3" :`true` "NewEnumerator2" :!type "/Game/Blueprints/Enum_Direction Enum") :`true` "NewEnumerator1") :`true` "NewEnumerator0")))
  (`PaperFlipbookComponent.SetFlipbook` (`self.PaperFlipbook`) (select `bool` (`self.isFalling`) :`false` (select `/Game/Blueprints/Enum_Direction` _directionenum :`NewEnumerator0` (`|GetArrayItem` _flipbook_array) :`NewEnumerator1` (`|GetArrayItem` _flipbook_array 1) :`NewEnumerator2` (`|GetArrayItem` _flipbook_array 2) :`NewEnumerator3` (`|GetArrayItem` _flipbook_array 3)) :`true` (select `/Game/Blueprints/Enum_Direction` _directionenum :`NewEnumerator0` (`|GetArrayItem` _flipbook_array 20) :`NewEnumerator1` (`|GetArrayItem` _flipbook_array 21) :`NewEnumerator2` (`|GetArrayItem` _flipbook_array 22) :`NewEnumerator3` (`|GetArrayItem` _flipbook_array 23)))))

(fn `P2Lifting`
  (params (ArrowUp :type "Float (double-precision)") (ArrowRight :type "Float (double-precision)"))
  (bind _flipbook_array (`self.Flipbook Array`))
  (bind _directionenum (`self.DirectionEnum`))
  (if (or (!= ArrowUp 0.0) (!= ArrowRight 0.0))
    (set `self.DirectionEnum` (select `bool` (> ArrowUp 0.0) :`false` (select `bool` (< ArrowUp 0.0) :`false` (select `bool` (> ArrowRight 0.0) :`false` "NewEnumerator3" :`true` "NewEnumerator2" :!type "/Game/Blueprints/Enum_Direction Enum") :`true` "NewEnumerator1") :`true` "NewEnumerator0")))
  (`PaperFlipbookComponent.SetFlipbook` (`self.PaperFlipbook`) (select `bool` (!= (`KismetMathLibrary.VSize` (`SceneComponent.GetComponentVelocity` (`self.Capsule`))) 0.0) :`false` (select `/Game/Blueprints/Enum_Direction` _directionenum :`NewEnumerator0` (`|GetArrayItem` _flipbook_array 8) :`NewEnumerator1` (`|GetArrayItem` _flipbook_array 9) :`NewEnumerator2` (`|GetArrayItem` _flipbook_array 10) :`NewEnumerator3` (`|GetArrayItem` _flipbook_array 11)) :`true` (select `/Game/Blueprints/Enum_Direction` _directionenum :`NewEnumerator0` (`|GetArrayItem` _flipbook_array 12) :`NewEnumerator1` (`|GetArrayItem` _flipbook_array 13) :`NewEnumerator2` (`|GetArrayItem` _flipbook_array 14) :`NewEnumerator3` (`|GetArrayItem` _flipbook_array 15)))))

(fn `P2Walking`
  (params (`Arrow Up` :type "Float (double-precision)") (`Arrow Right` :type "Float (double-precision)"))
  (bind _directionenum (`self.DirectionEnum`))
  (bind _flipbook_array (`self.Flipbook Array`))
  (if (or (!= `Arrow Up` 0.0) (!= `Arrow Right` 0.0))
    (set `self.isWalking` true)
    (set `self.DirectionEnum` (select `bool` (> `Arrow Up` 0.0) :`false` (select `bool` (< `Arrow Up` 0.0) :`false` (select `bool` (> `Arrow Right` 0.0) :`false` "NewEnumerator3" :`true` "NewEnumerator2" :!type "/Game/Blueprints/Enum_Direction Enum") :`true` "NewEnumerator1") :`true` "NewEnumerator0"))
    (else
      (set `self.isWalking` false)))
  (`PaperFlipbookComponent.SetFlipbook` (`self.PaperFlipbook`) (select `bool` (> (`KismetMathLibrary.VSize` (`SceneComponent.GetComponentVelocity` (`self.Capsule`))) 0.0) :`false` (select `/Game/Blueprints/Enum_Direction` _directionenum :`NewEnumerator0` (`|GetArrayItem` _flipbook_array) :`NewEnumerator1` (`|GetArrayItem` _flipbook_array 1) :`NewEnumerator2` (`|GetArrayItem` _flipbook_array 2) :`NewEnumerator3` (`|GetArrayItem` _flipbook_array 3)) :`true` (select `/Game/Blueprints/Enum_Direction` _directionenum :`NewEnumerator0` (`|GetArrayItem` _flipbook_array 4) :`NewEnumerator1` (`|GetArrayItem` _flipbook_array 5) :`NewEnumerator2` (`|GetArrayItem` _flipbook_array 6) :`NewEnumerator3` (`|GetArrayItem` _flipbook_array 7)))))

(fn `Play Flipbook`
  (params (ArrowUp :type "Float (double-precision)") (ArrowRight :type "Float (double-precision)"))
  (if (`self.isLifting`)
    (`self.P2Lifting` ArrowUp ArrowRight)
    (elif (`self.isAttacking`)
      (`self.P2Attack` ArrowUp ArrowRight)
      (elif (`self.isFalling`)
        (`self.P2Falling` ArrowUp ArrowRight)
        (else
          (`self.P2Walking` ArrowUp ArrowRight))))))

(fn `SetColor`
  (params (Selection :type "/Game/Blueprints/Enum_Flipbooks Enum" :default "NewEnumerator0"))
  (switch `/Game/Blueprints/Enum_Flipbooks` Selection
    (:`NewEnumerator0`
      (set `self.Flipbook Array` (`self.Red`)))
    (:`NewEnumerator1`
      (set `self.Flipbook Array` (`self.Green`)))
    (:`NewEnumerator2`
      (set `self.Flipbook Array` (`self.Blue`)))
    (:`NewEnumerator3`
      (set `self.Flipbook Array` (`self.Yellow`)))))

(fn `UserConstructionScript`)