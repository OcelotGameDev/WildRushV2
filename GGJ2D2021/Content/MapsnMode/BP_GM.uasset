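; BP_GM, apparently the game mode going by its name, holds an unfinished two-player shared camera and currently does nothing when run.
; BeginPlay, UpdateCamera and the construction script are empty.
; Disconnected nodes gather both player controllers, set view targets, cache player references from LevelCtrl and start a looping UpdateCamera timer.
; Other orphaned fragments scale camera arm length by clamped distance between players.
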(event `self.ReceiveBeginPlay`)

(event `UpdateCamera`)

(fn `UserConstructionScript`)